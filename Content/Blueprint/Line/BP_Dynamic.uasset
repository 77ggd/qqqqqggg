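; Geometry Script generated mesh actor that builds a box and bakes it into a static mesh asset.
; On rebuild of the generated mesh, it appends a box with per-face polygroups and uniform UVs, then copies the result to ToStaticMeshAsset.
; A successful copy calls SetStaticMeshCollisionFromComponent on that asset, with no source component specified.
; BeginPlay, Tick, overlap and construction logic are empty, and some unconnected mesh nodes remain.
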(event EventBeginPlay)

(event Collision|EventActorBeginOverlap
  (params (OtherActor :type Actor%20Object%20Reference)))

(event EventTick
  (params (DeltaSeconds :type Float%20%28single-precision%29)))

(event Events|EventOnRebuildGeneratedMesh
  (params (TargetMesh :type Dynamic%20Mesh%20Object%20Reference))
  (bind _to_static_mesh_asset (Variables|Default|GetTo%20Static%20Mesh%20Asset))
  (bind _returnvalue (Class|GeometryScriptLibraryMeshPrimitiveFunctions|AppendBox TargetMesh (Utilities|Struct|MakeGeometryScriptPrimitiveOptions "PerFace") (Math|Transform|MakeTransform "0, 0, 0" "0, 0, 0" "1.000000,1.000000,1.000000") 1e+02 1e+02 1e+02 0 0 0 "Base" 0))
  (GeometryScript|StaticMesh|CopyMeshtoStaticMesh :FromDynamicMesh _returnvalue :ToStaticMeshAsset _to_static_mesh_asset :Debug 0
    (:Success
      (Class|GeometryScriptLibraryCollisionFunctions|SetStaticMeshCollisionfromComponent _to_static_mesh_asset 0 (Utilities|Struct|MakeGeometryScriptSetSimpleCollisionOptions true) 0))))

(fn ConstructionScript)