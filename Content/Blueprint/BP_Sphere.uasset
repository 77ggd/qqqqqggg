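; BP_Sphere is a trigger volume that follows the player and reveals or hides nearby BP_Animation actors.
; Each tick it moves, without sweeping, to the location of player pawn 0.
; Its Sphere component calls Show on BP_Animation actors that begin overlapping and Disappear on those that leave.
; The construction script sizes the sphere from the SphereRadius variable.
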(event OnComponentBeginOverlap(Sphere)
  (params (OverlappedComponent :type Primitive%20Component%20Object%20Reference) (OtherActor :type Actor%20Object%20Reference) (OtherComp :type Primitive%20Component%20Object%20Reference) (OtherBodyIndex :type Integer) (bFromSweep :type Boolean) (SweepResult :type Hit%20Result%20Structure%20%28by%20ref%29))
  (bind _asbp_animation (Utilities|Casting|CastToBP_Animation OtherActor))
  (Default|Show _asbp_animation))

(event OnComponentEndOverlap(Sphere)
  (params (OverlappedComponent :type Primitive%20Component%20Object%20Reference) (OtherActor :type Actor%20Object%20Reference) (OtherComp :type Primitive%20Component%20Object%20Reference) (OtherBodyIndex :type Integer))
  (bind _asbp_animation (Utilities|Casting|CastToBP_Animation OtherActor))
  (Default|Disappear _asbp_animation))

(event EventBeginPlay)

(event Collision|EventActorBeginOverlap
  (params (OtherActor :type Actor%20Object%20Reference)))

(event EventTick
  (params (DeltaSeconds :type Float%20%28single-precision%29))
  (Transformation|SetActorLocation (Transformation|GetActorLocation (Game|Player|GetPlayerPawn 0)) false false))

(fn ConstructionScript
  (Components|Sphere|SetSphereRadius (Variables|Default|GetSphere) (Variables|Default|GetSphere%20Radius) true))