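; BP_Line is a spline actor that positions a referenced actor along its path and can extend that path from the player character's position.
; AddActor and ClearActor set or clear the actor reference, and AddPoint appends a world-space spline point at the BP_ThirdPersonCharacter's location.
; The construction script places the actor at the Location fraction of spline length, rotated to the tangent.
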(event Custom|Add%20Point
  (bind _returnvalue (Actor|GetActorOfClass "/Game/ThirdPerson/Blueprints/BP_ThirdPersonCharacter.BP_ThirdPersonCharacter_C"))
  (Spline|AddSplinePoint (Variables|Default|GetSpline) (Transformation|GetActorLocation _returnvalue) "World" true))

(event Custom|Add%20Actor
  (params (Actor :type Actor%20Object%20Reference))
  (Variables|Default|SetActor Actor))

(event Custom|Clear%20Actor
  (Variables|Default|SetActor 0))

(event EventBeginPlay)

(event Collision|EventActorBeginOverlap
  (params (OtherActor :type Actor%20Object%20Reference)))

(event EventTick
  (params (DeltaSeconds :type Float%20%28single-precision%29)))

(fn ConstructionScript
  (bind _spline (Variables|Default|GetSpline))
  (bind _location (Variables|Default|GetLocation))
  (bind _spline_2 (Variables|Default|GetSpline))
  (bind _returnvalue (Spline|GetSplineLength _spline))
  (bind _returnvalue_2 (* _returnvalue _location))
  (Transformation|SetActorLocationAndRotation (Variables|Default|GetActor) (Spline|GetLocationatDistanceAlongSpline _spline_2 _returnvalue_2 "World") (Math|Conversions|RotationFromXVector (Spline|GetTangentatDistanceAlongSpline _spline_2 _returnvalue_2 "World"))))