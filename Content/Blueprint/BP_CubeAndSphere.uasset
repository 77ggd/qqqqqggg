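; BP_CubeAndSphere is an actor that animates the material and vertical movement of its Sphere component.
; A looping 10-second timer alternates a timeline between play and reverse, feeding its track to the "Fade Amount" and "Color" scalar material parameters.
; Tick moves the Sphere along Z by a fixed, frame-rate-dependent step signed by IsUp.
; IsUp flips only when the timeline value exactly equals 0.5, a fragile float comparison.
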(event Custom|Color%20And%20Float
  (bind _sphere (Variables|Default|GetSphere))
  (Utilities|FlowControl|FlipFlop
    (:A
      (bind _新建轨道_0 (Timeline|时间轴 Play)
        (:Update
          (Rendering|Material|SetScalarParameterValueonMaterials _sphere "Fade Amount" _新建轨道_0)
          (Rendering|Material|SetScalarParameterValueonMaterials _sphere "Color" _新建轨道_0)
          (if (== _新建轨道_0 0.5)
            (Variables|Default|SetIs%20Up? (* (Variables|Default|GetIs%20Up?) -1))))))
    (:B
      (Timeline|时间轴 Reverse))))

(event EventBeginPlay
  (Utilities|Time|SetTimerbyEvent (delegate Custom|Color%20And%20Float) 1e+01 true))

(event Collision|EventActorBeginOverlap
  (params (OtherActor :type Actor%20Object%20Reference)))

(event EventTick
  (params (DeltaSeconds :type Float%20%28single-precision%29))
  (bind _sphere (Variables|Default|GetSphere))
  (bind _returnvalue (Transformation|GetWorldLocation _sphere))
  (Transformation|SetWorldLocation _sphere (Math|Vector|MakeVector (.x _returnvalue) (.y _returnvalue) (+ (.z _returnvalue) (* 2 (Variables|Default|GetIs%20Up?)))) false false))

(fn ConstructionScript)