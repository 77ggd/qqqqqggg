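; BP_Animation is an actor that animates itself in and out by scaling.
; It starts hidden and caches its scale at BeginPlay; Show unhides it and plays a timeline that lerps scale from zero to that cached value.
; Disappear reverses the timeline without re-hiding the actor.
; Two DoOnce gates reset each other, so repeated Show or Disappear calls are ignored until the opposite event fires.
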(event Custom|Show
  (Utilities|FlowControl|Sequence
    (:then_0
      (Utilities|FlowControl|DoOnce false
        (:Completed
          (Rendering|SetActorHiddenInGame false)
          (bind _scale (Timeline|时间轴 Play)
            (:Update
              (Transformation|SetActorScale3D (Math|Vector|Lerp(Vector) "0, 0, 0" (Variables|Default|GetScale) _scale)))))))
    (:then_1
      (Utilities|FlowControl|DoOnce false) ; enters at Reset
    )))

(event Custom|Disappear
  (Utilities|FlowControl|Sequence
    (:then_0
      (Utilities|FlowControl|DoOnce false
        (:Completed
          (bind _scale (Timeline|时间轴 Reverse)
            (:Update
              (Transformation|SetActorScale3D (Math|Vector|Lerp(Vector) "0, 0, 0" (Variables|Default|GetScale) _scale)))))))
    (:then_1
      (Utilities|FlowControl|DoOnce false) ; enters at Reset
    )))

(event EventBeginPlay
  (Variables|Default|SetScale (Transformation|GetActorScale3D)))

(event Collision|EventActorBeginOverlap
  (params (OtherActor :type Actor%20Object%20Reference)))

(event EventTick
  (params (DeltaSeconds :type Float%20%28single-precision%29)))

(fn ConstructionScript
  (Rendering|SetActorHiddenInGame true))